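; Actor component that stamps footprints into a render target window that follows its owner and spawns wet or dry footstep Niagara effects.
; Tick scrolls the ping-ponged buffers by texel-snapped movement through a material and parameter collection, while decaying carried wetness.
; Footstep events look up surface data, sample the landscape's "Wet" layer to update wetness, then draw an oriented, left/right-flipped brush into both buffers.
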(event `self.ReceiveBeginPlay`
  ; Begin Play
  (`KismetRenderingLibrary.ClearRenderTarget2D` (`self.RT_FootprintBuffer_A`))
  (`KismetRenderingLibrary.ClearRenderTarget2D` (`self.RT_FootprintBuffer_B`))
  (set `self.Owner` (`self.GetOwner`))
  (bind _output_get (set `self.CharacterLocation` (`Actor.K2_GetActorLocation` (`self.Owner`))))
  (set `self.LastCharacterPosition` _output_get)
  (bind _returnvalue (`GameplayStatics.GetActorOfClass` "/Script/Landscape.LandscapeProxy"))
  (set `self.Landscape` _returnvalue)
  (`KismetMaterialLibrary.SetScalarParameterValue` "/WetFootprintSystem/Materials/MPC_FootprintData.MPC_FootprintData" "LocalRTSize" (`self.LocalRTSize`))
  (bind _returnvalue_2 (`KismetMaterialLibrary.CreateDynamicMaterialInstance` "/WetFootprintSystem/Materials/M_FootprintUpdate.M_FootprintUpdate" "None"))
  (set `self.ScrollDMI` _returnvalue_2)
  (`KismetMaterialLibrary.SetScalarParameterValue` "/WetFootprintSystem/Materials/MPC_FootprintData.MPC_FootprintData" "CharacterPos_X" (.x (`Actor.K2_GetActorLocation` (`self.Owner`))))
  (`KismetMaterialLibrary.SetScalarParameterValue` "/WetFootprintSystem/Materials/MPC_FootprintData.MPC_FootprintData" "CharacterPos_Y" (.y (`Actor.K2_GetActorLocation` (`self.Owner`))))
  (set `self.CurrentRT` (`self.RT_FootprintBuffer_A`))
  (set `self.PreviousRT` (`self.RT_FootprintBuffer_B`)))

(event `self.ReceiveTick`
  (params (DeltaSeconds :type "Float (single-precision)"))
  (bind _rtsize (`self.RTSize`))
  (bind _localrtsize (`self.LocalRTSize`))
  (bind _rtsize_2 (`self.RTSize`))
  (bind _returnvalue (`Actor.K2_GetActorLocation` (`self.Owner`)))
  ; Tick
  (set `self.WetnessLevel` (`KismetMathLibrary.FClamp` (- (`self.WetnessLevel`) (* DeltaSeconds 0.05 (`self.DryingRate`)))))
  (set `self.CharacterLocation` (`Actor.K2_GetActorLocation` (`self.Owner`)))
  (`KismetMaterialLibrary.SetScalarParameterValue` "/WetFootprintSystem/Materials/MPC_FootprintData.MPC_FootprintData" "ScrollOffset_X" (/ (`KismetMathLibrary.Round` (* (/ (.x (- (`self.CharacterLocation`) (`self.LastCharacterPosition`))) _localrtsize) _rtsize)) _rtsize_2))
  (`KismetMaterialLibrary.SetScalarParameterValue` "/WetFootprintSystem/Materials/MPC_FootprintData.MPC_FootprintData" "ScrollOffset_Y" (/ (`KismetMathLibrary.Round` (* (/ (.y (- (`self.CharacterLocation`) (`self.LastCharacterPosition`))) _localrtsize) _rtsize)) _rtsize_2))
  (`MaterialInstanceDynamic.SetTextureParameterValue` (`self.ScrollDMI`) "PreviousRT" (`self.PreviousRT`))
  (`KismetRenderingLibrary.DrawMaterialToRenderTarget` (`self.CurrentRT`) (`self.ScrollDMI`))
  (set `self.Temp` (`self.CurrentRT`))
  (set `self.CurrentRT` (`self.PreviousRT`))
  (set `self.PreviousRT` (`self.Temp`))
  (set `self.LastCharacterPosition` _returnvalue)
  (`KismetMaterialLibrary.SetScalarParameterValue` "/WetFootprintSystem/Materials/MPC_FootprintData.MPC_FootprintData" "CharacterPos_X" (.x _returnvalue))
  (`KismetMaterialLibrary.SetScalarParameterValue` "/WetFootprintSystem/Materials/MPC_FootprintData.MPC_FootprintData" "CharacterPos_Y" (.y _returnvalue)))

(event `/WetFootprintSystem/Blueprints/BPI_SurfaceResponse.HandleFootstep`
  (params (IsLeftFoot :type Boolean) (HitResult :type "HitResult Structure"))
  (bind (_bblockinghit _binitialoverlap _time _distance _location _impactpoint _normal _impactnormal _physmat) (`GameplayStatics.BreakHitResult` HitResult))
  (bind (_x _y) (`self.Calculate UV`))
  (bind (_returnvalue_roll _returnvalue_pitch _returnvalue_yaw) (`KismetMathLibrary.BreakRotator` (`Actor.K2_GetActorRotation` (`self.Owner`))))
  (bind _returnvalue (`KismetMathLibrary.DegreesToRadians` (+ _returnvalue_yaw 90.0)))
  ; Handle Footstep
  (set `self.IsLeftFoot` IsLeftFoot)
  (set `self.HitLocation` _location)
  (set `self.HitNormal` _normal)
  (bind _returnvalue_2 (`|GetDataTableRow` "/WetFootprintSystem/Blueprints/DT_FootprintData.DT_FootprintData" (`|GetEnumeratorName` (`PhysicalMaterial.SurfaceType` _physmat)))
    (:`then`
      (bind (_drynormalstrength _wetnormalstrength _dryniagarasystem _wetniagarasystem) (break `/WetFootprintSystem/Blueprints/FS_FootprintData` _returnvalue_2))
      (`KismetMaterialLibrary.SetScalarParameterValue` "/WetFootprintSystem/Materials/MPC_FootprintData.MPC_FootprintData" "DryNormalStrength" _drynormalstrength)
      (`KismetMaterialLibrary.SetScalarParameterValue` "/WetFootprintSystem/Materials/MPC_FootprintData.MPC_FootprintData" "WetnessNormalStrength" _wetnormalstrength)
      (bind _returnvalue_3 (`LandscapeWeightLibrary.GetLandscapeLayerWeightAtLocation` (`self.Landscape`) (`self.HitLocation`) "Wet"))
      (set `self.GroundWetness` _returnvalue_3)
      (if (> (`self.GroundWetness`) (`self.WetnessLevel`))
        (set `self.WetnessLevel` (`self.GroundWetness`))
        (else
          (set `self.WetnessLevel` (`KismetMathLibrary.Lerp` (`self.WetnessLevel`) (`self.GroundWetness`) (`self.DryingRate`)))))
      (`KismetSystemLibrary.PrintString` (`KismetStringLibrary.Concat_StrStr` "Wetness Level: " (`KismetStringLibrary.Conv_DoubleToString` (`self.WetnessLevel`))))
      (`KismetSystemLibrary.PrintString` (`KismetStringLibrary.Concat_StrStr` "Ground Wetness: " (`KismetStringLibrary.Conv_DoubleToString` (`self.GroundWetness`))))
      (if (< (`self.GroundWetness`) 0.01)
        (`NiagaraFunctionLibrary.SpawnSystemAtLocation` _dryniagarasystem (`self.HitLocation`) (`KismetMathLibrary.MakeRotFromZ` (`self.HitNormal`)) (2.0 2.0 2.0))
        (else
          (bind _returnvalue_4 (`NiagaraFunctionLibrary.SpawnSystemAtLocation` _wetniagarasystem (`self.HitLocation`) (`KismetMathLibrary.MakeRotFromZ` (`self.HitNormal`)) (2.0 2.0 2.0)))
          (`NiagaraComponent.SetVariableFloat` _returnvalue_4 "WetnessIntensity" (`self.GroundWetness`))))
      (`KismetMaterialLibrary.SetScalarParameterValue` "/WetFootprintSystem/Materials/MPC_FootprintData.MPC_FootprintData" "WetnessLevel" (`self.WetnessLevel`))
      (`KismetMaterialLibrary.SetScalarParameterValue` "/WetFootprintSystem/Materials/MPC_FootprintData.MPC_FootprintData" "FootprintUV_X" _x)
      (`KismetMaterialLibrary.SetScalarParameterValue` "/WetFootprintSystem/Materials/MPC_FootprintData.MPC_FootprintData" "FootprintUV_Y" _y)
      (`KismetMaterialLibrary.SetScalarParameterValue` "/WetFootprintSystem/Materials/MPC_FootprintData.MPC_FootprintData" "FootprintCos" (`KismetMathLibrary.Cos` _returnvalue))
      (`KismetMaterialLibrary.SetScalarParameterValue` "/WetFootprintSystem/Materials/MPC_FootprintData.MPC_FootprintData" "FootprintSin" (* (`KismetMathLibrary.Sin` _returnvalue) -1.0))
      (`KismetMaterialLibrary.SetScalarParameterValue` "/WetFootprintSystem/Materials/MPC_FootprintData.MPC_FootprintData" "FootprintFlip" (select `bool` (`self.IsLeftFoot`) :`false` 1.0 :!type "Float (single-precision)"))
      (`KismetRenderingLibrary.DrawMaterialToRenderTarget` (`self.CurrentRT`) (`self.M_FootprintBrush`))
      (`KismetRenderingLibrary.DrawMaterialToRenderTarget` (`self.PreviousRT`) (`self.M_FootprintBrush`)))))